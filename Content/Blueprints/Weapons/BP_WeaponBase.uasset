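; Base weapon Blueprint that handles magazine ammo, firing and reloading, with an empty WeaponTrace event as the hit hook.
; FireWeapon spends a round, spawns muzzle emitter and sound at the Arrow, calls WeaponTrace, and auto-reloads on an empty magazine.
; Manual and automatic reloads share a DoOnce gate that shows a reload-bar widget, waits ReloadTime, then refills Ammo.
; It also exposes an FOV multiplier through a getter.
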(event `WeaponTrace`)

(event `self.ReceiveBeginPlay`
  (set `self.ammo` (`self.MaxMagazineAmmo`)))

(event `/Game/Blueprints/FirstPersonTemplate/Bpi_Weapon.FireWeapon`
  (`/Game/Blueprints/Libraries/BPML_Comparisons.INT<=INT` (`self.ammo`)
    (:`True`
      (`self.ReloadWeapon`))
    (:`False`
      (set `self.ammo` (- (`self.ammo`) 1))
      (`self.weaponFireEffects`)
      (`self.WeaponTrace`)
      (`/Game/Blueprints/Libraries/BPML_Comparisons.INT<=INT` (`self.ammo`)
        (:`True`
          (`self.ReloadWeapon`))))))

(event `ReloadWeapon`
  ;[1 0.1128 0.5751] Reload Animation
  (`/Engine/EditorBlueprintResources/StandardMacros.DoOnce` false :!label _label
    (:`Completed`
      (bind _returnvalue (`|CreateWidget` "/Game/Blueprints/Weapons/WB_ReloadBar.WB_ReloadBar_C"))
      (`/Game/Blueprints/Weapons/WB_ReloadBar.ReloadAnimation` _returnvalue (`self.ReloadTime`))
      (`UserWidget.AddToViewport` _returnvalue 0)
      (`KismetSystemLibrary.Delay` (`self.ReloadTime`))
      (set `self.ammo` (`self.MaxMagazineAmmo`))
      (goto _label :!via `Reset`))))

(event `/Game/Blueprints/FirstPersonTemplate/Bpi_Weapon.Reload`
  ;[1 0.1128 0.5751] Reload Animation
  (goto _label))

(fn `GetFOVMultiplier`
  (returns (`FOV Multiplier` :type "Float (double-precision)"))
  (return (`self.FOV Multiplier`)))

(fn `UserConstructionScript`)

(fn `weaponFireEffects`
  (bind (_returnvalue_location _returnvalue_rotation) (`KismetMathLibrary.BreakTransform` (`SceneComponent.K2_GetComponentToWorld` (`self.Arrow`))))
  ;[0 0.6893 1] Weapon soudeffects and shotting effects
  (`GameplayStatics.SpawnEmitterAtLocation` (`self.Weapon Fire Emiter`) _returnvalue_location _returnvalue_rotation (`self.Weapon Fire Emiter Scale`))
  (`GameplayStatics.SpawnSoundAtLocation` (`self.Weapon Fire Sound`) _returnvalue_location (struct) 1.0 1.0 0.0 null null)
  (return))