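; BP_WeaponSwap is an interactable actor that changes the weapon held by the first-person player.
; Its construction script sets the BPWeapon child actor to the Weapon class variable, so each instance displays the weapon it grants.
; On Interacted, it casts player character 0 to BP_FirstPersonCharacter and sets that character's Weapon child actor to the same class.
; The actor itself stays unchanged after the swap.
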(event `self.Interacted`
  (bind _asbp_first_person_character (cast `/Game/Blueprints/FirstPersonTemplate/BP_FirstPersonCharacter` (`GameplayStatics.GetPlayerCharacter` 0)))
  (`ChildActorComponent.SetChildActorClass` (`/Game/Blueprints/FirstPersonTemplate/BP_FirstPersonCharacter.Weapon` _asbp_first_person_character) (`self.Weapon`)))

(fn `UserConstructionScript`
  (`parent.UserConstructionScript`)
  (`ChildActorComponent.SetChildActorClass` (`self.BP_Weapon`) (`self.Weapon`)))