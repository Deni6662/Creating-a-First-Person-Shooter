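; Shootable target actor with randomized size and behavior that awards score to its spawner when damaged.
; The construction script rolls scale and behavior; BeginPlay sets a random timeline speed and, for movers, a random offset.
; The timeline lerps the mesh along relative X or Y ("vertical" uses Y) or grows its scale.
; RecieveDamage reports clamped points to SpawnerRefrence, plays explosion sound and particles, then destroys the actor.
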(event `self.ReceiveBeginPlay`
  (bind _returnvalue (`KismetMathLibrary.RandomFloatInRange` 100.0 1000.0))
  (bind _randomscale (`self.RandomScale`))
  (bind _returnvalue_2 (* _randomscale 1.5))
  ;[0.1086 1 0.1225] Random Generation of behavior
  (switch `/Game/Blueprints/Target/E_TargetBehavior` (`self.E_Target Behavior`)
    (:`NewEnumerator1`
      (set `self.Destination_Location` (`KismetMathLibrary.MakeVector` _returnvalue)))
    (:`NewEnumerator2`
      (set `self.Destination_Location` (`KismetMathLibrary.MakeVector` 0.0 _returnvalue)))
    (:`NewEnumerator3`
      _))
  (`TimelineComponent.SetPlayRate` (`self.T_movement`) (/ 1.0 (`KismetMathLibrary.RandomFloatInRange` 2.0 4.0)))
  (bind (_direction _alpha) (`Timeline|T_movement` :!via `PlayFromStart`)
    (:`Update`
      (switch `/Game/Blueprints/Target/E_TargetBehavior` (`self.E_Target Behavior`)
        (:`NewEnumerator1`
          (`SceneComponent.K2_SetRelativeLocation` (`self.SM_target`) (`KismetMathLibrary.VLerp` (0.0 0.0 0.0) (`self.Destination_Location`) _alpha) false false :!label _label))
        (:`NewEnumerator2`
          (goto _label))
        (:`NewEnumerator3`
          (`SceneComponent.SetWorldScale3D` (`self.SM_target`) (`KismetMathLibrary.VLerp` (`KismetMathLibrary.MakeVector` _randomscale _randomscale _randomscale) (`KismetMathLibrary.MakeVector` _returnvalue_2 _returnvalue_2 _returnvalue_2) _alpha)))))))

(event `/Game/Blueprints/Weapons/BPI_Damage.Recieve Damage`
  (params (Points :type Integer))
  (bind _returnvalue (`SceneComponent.K2_GetComponentLocation` (`self.SM_target`)))
  (`/Game/Blueprints/Target/BP_TargetSpawner.UpdateMatchScore` (`self.SpawnerRefrence`) (`KismetMathLibrary.Clamp` Points 1 5))
  (`GameplayStatics.SpawnSoundAtLocation` "/Game/StarterContent/Audio/Explosion_Cue.Explosion_Cue" _returnvalue (struct) 1.0 1.0 0.0 null null)
  (`GameplayStatics.SpawnEmitterAtLocation` "/Game/StarterContent/Particles/P_Explosion.P_Explosion" _returnvalue (struct) (0.2 0.2 0.2))
  (`self.K2_DestroyActor`))

(fn `UserConstructionScript`
  (bind _output_get (set `self.RandomScale` (`KismetMathLibrary.RandomFloatInRange` 0.25 1.0)))
  (`SceneComponent.SetWorldScale3D` (`self.SM_target`) (`KismetMathLibrary.MakeVector` _output_get _output_get _output_get))
  (set `self.E_Target Behavior` (cast `/Game/Blueprints/Target/E_TargetBehavior` (`KismetMathLibrary.Conv_IntToByte` (`KismetMathLibrary.RandomIntegerInRange` 1 3)))))