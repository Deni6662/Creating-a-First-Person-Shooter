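; Target spawner for an aim trainer that runs a one-shot timed round with music and tracks match score.
; Start_Spawning spawns an initial burst, then a looping timer adds capped, camera-facing BP_Targets at random points in a construction-sized box.
; Targets receive a spawner reference; UpdateMatchScore accumulates points into the WB_Score widget.
; At round end it clears targets, updating session high in GI_AimTrainer and all-time high in a SaveGame slot.
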(event `UpdateMatchScore`
  (params (Points :type Integer))
  (bind _output_get (set `self.MatchPoints` (+ Points (`self.MatchPoints`))))
  (`TextBlock.SetText` (`/Game/Blueprints/Target/WB_Score.CurrentScore` (`self.WB Score`)) (`KismetTextLibrary.Conv_IntToText` _output_get)))

(event `self.ReceiveBeginPlay`
  ;[0 0.7774 1] Beggin Play
  (bind _returnvalue (`|CreateWidget` "/Game/Blueprints/Target/WB_Score.WB_Score_C"))
  (bind _output_get (set `self.WB Score` _returnvalue))
  (`UserWidget.AddToViewport` (`self.WB Score`) 0)
  (`UserWidget.AddToViewport` _output_get 0)
  (`|ExecutionSequence`
    (:`then_0`
      (bind _asgi_aim_trainer (cast `/Game/Blueprints/FirstPersonTemplate/GI_AimTrainer` (`GameplayStatics.GetGameInstance`)))
      (`TextBlock.SetText` (`/Game/Blueprints/Target/WB_Score.SessionHigh` (`self.WB Score`)) (`KismetTextLibrary.Conv_IntToText` (`/Game/Blueprints/FirstPersonTemplate/GI_AimTrainer.Score` _asgi_aim_trainer))))
    (:`then_1`
      (bind _returnvalue_2 (`GameplayStatics.DoesSaveGameExist` "Score"))
      (if _returnvalue_2
        (bind _returnvalue_3 (`GameplayStatics.LoadGameFromSlot` "Score"))
        (bind _asbps_aim_trainer_save (cast `/Game/Blueprints/FirstPersonTemplate/BPS_AimTrainer_Save` _returnvalue_3))
        (`TextBlock.SetText` (`/Game/Blueprints/Target/WB_Score.AllTimeHigh` (`self.WB Score`)) (`KismetTextLibrary.Conv_IntToText` (`/Game/Blueprints/FirstPersonTemplate/BPS_AimTrainer_Save.HighScore` _asbps_aim_trainer_save)))
        (else
          (bind _returnvalue_4 (`GameplayStatics.CreateSaveGameObject` "/Game/Blueprints/FirstPersonTemplate/BPS_AimTrainer_Save.BPS_AimTrainer_Save_C"))
          (`GameplayStatics.SaveGameToSlot` _returnvalue_4 "Score"))))))

(event `Start_Spawning`
  (bind _matchpoints (`self.MatchPoints`))
  (bind _matchpoints_2 (`self.MatchPoints`))
  ;[0 0.7186 1] Start Spawning Targets
  (`/Engine/EditorBlueprintResources/StandardMacros.DoOnce` false
    (:`Completed`
      (bind _returnvalue (`GameplayStatics.SpawnSound2D` "/Game/Blueprints/Soudtrack/Escala.Escala" 1.0 1.0 0.0 null))
      (set `self.AimTrainerMusic` _returnvalue)
      (`AudioComponent.FadeIn` _returnvalue 1.0 0.3 0.0 "Linear")
      (bind _returnvalue_2 (`KismetSystemLibrary.K2_SetTimerDelegate` (delegate `SpawnTarget`) 1.0 true))
      (set `self.Target Spawner` _returnvalue_2)
      (for _ (range 9)
        (`self.SpawnTarget`))
      (`KismetSystemLibrary.Delay` 10.0)
      (`KismetSystemLibrary.K2_ClearAndInvalidateTimerHandle` (`self.Target Spawner`))
      (bind _outactors (`GameplayStatics.GetAllActorsOfClass` "/Game/Blueprints/Target/BP_Target.BP_Target_C"))
      (for _array_element _outactors
        (`self.K2_DestroyActor` _array_element))
      (`|ExecutionSequence`
        (:`then_0`
          (bind _asgi_aim_trainer (cast `/Game/Blueprints/FirstPersonTemplate/GI_AimTrainer` (`GameplayStatics.GetGameInstance`)))
          (if (> _matchpoints_2 (`/Game/Blueprints/FirstPersonTemplate/GI_AimTrainer.Score` _asgi_aim_trainer))
            (bind _output_get (set `/Game/Blueprints/FirstPersonTemplate/GI_AimTrainer.Score` _matchpoints_2 _asgi_aim_trainer))
            (`TextBlock.SetText` (`/Game/Blueprints/Target/WB_Score.SessionHigh` (`self.WB Score`)) (`KismetTextLibrary.Conv_IntToText` _output_get))))
        (:`then_1`
          (bind _returnvalue_3 (`GameplayStatics.LoadGameFromSlot` "Score"))
          (bind _asbps_aim_trainer_save (cast `/Game/Blueprints/FirstPersonTemplate/BPS_AimTrainer_Save` _returnvalue_3))
          (if (< (`/Game/Blueprints/FirstPersonTemplate/BPS_AimTrainer_Save.HighScore` _asbps_aim_trainer_save) _matchpoints)
            (`TextBlock.SetText` (`/Game/Blueprints/Target/WB_Score.AllTimeHigh` (`self.WB Score`)) (`KismetTextLibrary.Conv_IntToText` _matchpoints))
            (set `/Game/Blueprints/FirstPersonTemplate/BPS_AimTrainer_Save.HighScore` _matchpoints _asbps_aim_trainer_save)
            (`GameplayStatics.SaveGameToSlot` _asbps_aim_trainer_save "Score")))
        (:`then_2`
          (`AudioComponent.FadeOut` (`self.AimTrainerMusic`) 1.0 0.0 "Linear"))))))

(event `SpawnTarget`
  (bind _spawm_area (`self.Spawm_Area`))
  ;[0.9521 0 1] Changes to spawner variables such as size and rotation
  (bind _outactors (`GameplayStatics.GetAllActorsOfClass` "/Game/Blueprints/Target/BP_Target.BP_Target_C"))
  (if (<= (`KismetArrayLibrary.Array_Length` _outactors) 10)
    (bind _output_get (set `self.SpawnLocation` (`KismetMathLibrary.RandomPointInBoundingBox` (`SceneComponent.K2_GetComponentLocation` _spawm_area) (`BoxComponent.GetScaledBoxExtent` _spawm_area))))
    (bind (_returnvalue_roll _returnvalue_pitch _returnvalue_yaw) (`KismetMathLibrary.BreakRotator` (`KismetMathLibrary.FindLookAtRotation` _output_get (`SceneComponent.K2_GetComponentLocation` (`PlayerCameraManager.TransformComponent` (`GameplayStatics.GetPlayerCameraManager` 0))))))
    (`|SpawnActorFromClass` "/Game/Blueprints/Target/BP_Target.BP_Target_C" (`KismetMathLibrary.MakeTransform` _output_get (`KismetMathLibrary.MakeRotator` _returnvalue_roll _returnvalue_pitch (- _returnvalue_yaw 90.0))) "AdjustIfPossibleButAlwaysSpawn" "OverrideRootScale" null self null)))

(fn `UserConstructionScript`
  (`BoxComponent.SetBoxExtent` (`self.Spawm_Area`) (`self.In Box Extent`) true))